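; BP_ItemParent is the base Blueprint for world items that can be interacted with and picked up.
; Interact passes the instigator to ItemDataComponent's PickUpItem, with a short fixed hold time reported for the interaction.
; The prompt text is built from the item's Name, looked up in the data table through the component's ItemID row handle.
; SetOutlineState toggles Render Custom Depth on the static mesh to show or hide an outline.
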(event `/Game/Components/InteractionSystem/BPI_Interact.SetOutlineState`
  (params (`bShow?` :type Boolean))
  (bind _staticmesh (`self.StaticMesh`))
  (if `bShow?`
    (`PrimitiveComponent.SetRenderCustomDepth` _staticmesh true)
    (else
      (`PrimitiveComponent.SetRenderCustomDepth` _staticmesh false))))

(event `/Game/Components/InteractionSystem/BPI_Interact.Interact`
  (params (Instigator :type "Actor Object Reference"))
  (`/Game/Components/InventorySystem/ItemDataComponent.PickUpItem` (`self.ItemDataComponent`) Instigator))

(fn `GetInteractHoldTime`
  (returns (HoldTime :type "Float (double-precision)"))
  (return 0.5))

(fn `GetInteractText`
  (returns (InteractText :type Text))
  (bind (_itemid_datatable _itemid_rowname) (break `DataTableRowHandle` (`/Game/Components/InventorySystem/ItemDataComponent.ItemID` (`self.ItemDataComponent`))))
  (bind _returnvalue (`|GetDataTableRow` _itemid_datatable _itemid_rowname)
    (:`then`
      (return (`|FormatText` "Pick up {Item}" (`.Name_2_C5520A394930424370BD6BA562AAAB8A` (break `/Game/Components/InventorySystem/FItemStruct` _returnvalue)))))))

(fn `UserConstructionScript`)