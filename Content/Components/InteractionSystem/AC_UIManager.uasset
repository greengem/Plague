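; AC_UIManager is a UI manager component that shows the cursor and interaction prompt widgets.
; On BeginPlay it caches the player character's InteractionSystem_Base component and adds a cursor widget to the viewport.
; Each tick it polls that component's current hit, creating a prompt with the hit actor's interact text, updating its hold-progress timer, and removing it once the hit is lost.
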(event `self.ReceiveBeginPlay`
  (set `self.InteractionComponent` (`Actor.GetComponentByClass` (`GameplayStatics.GetPlayerCharacter` 0) "/Game/Components/InteractionSystem/InteractionSystem_Base.InteractionSystem_Base_C"))
  (bind _returnvalue (`|CreateWidget` "/Game/Components/InteractionSystem/UI/WB_Cursor.WB_Cursor_C" (`GameplayStatics.GetPlayerController` 0)))
  (`UserWidget.AddToViewport` _returnvalue 0))

(event `self.ReceiveTick`
  (params (DeltaSeconds :type "Float (single-precision)"))
  (`self.ShowInteractPrompt`))

(fn `ShowInteractPrompt`
  (bind _interactioncomponent (`self.InteractionComponent`))
  (bind _interactprompt (`self.InteractPrompt`))
  (bind (_returnvalue _currenthitactor) (`/Game/Components/InteractionSystem/InteractionSystem_Base.GetCurrentHit` (`self.InteractionComponent`)))
  (if _returnvalue
    (`/Engine/EditorBlueprintResources/StandardMacros.IsValid` (`self.InteractPrompt`)
      (:`Is Valid`
        _)
      (:`Is Not Valid`
        (bind _interacttext (message `/Game/Components/InteractionSystem/BPI_Interact.GetInteractText` _currenthitactor))
        (bind _returnvalue_2 (`|CreateWidget` "/Game/Components/InteractionSystem/UI/WB_InteractionPrompt.WB_InteractionPrompt_C" (`GameplayStatics.GetPlayerController` 0) _interacttext))
        (bind _output_get (set `self.InteractPrompt` _returnvalue_2))
        (`UserWidget.AddToViewport` _output_get 0)))
    (`/Game/Components/InteractionSystem/UI/WB_InteractionPrompt.UpdateTimer` (`self.InteractPrompt`) (/ (`/Game/Components/InteractionSystem/InteractionSystem_Base.CurrentHoldDuration` _interactioncomponent) (`/Game/Components/InteractionSystem/InteractionSystem_Base.InteractHoldTimer` _interactioncomponent)))
    (else
      (`/Engine/EditorBlueprintResources/StandardMacros.IsValid` _interactprompt
        (:`Is Valid`
          (`Widget.RemoveFromParent` _interactprompt)
          (set `self.InteractPrompt` null))))))