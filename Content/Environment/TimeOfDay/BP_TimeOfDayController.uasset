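; Time-of-day controller that switches the level's sun between morning, afternoon, evening and night presets through four debug keys.
; On BeginPlay it waits briefly, then caches the DirectionalLight it finds in the level.
; Each preset function instantly sets that light's rotation and intensity, with night turning intensity to zero; there is no blending or time progression.
; Every key press also prints a placeholder debug message.
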(event EventBeginPlay
  (Utilities|FlowControl|Delay 0.2)
  (bind _returnvalue (Actor|GetActorOfClass "/Script/Engine.DirectionalLight"))
  (Variables|Default|SetDirectionalLight_Ref _returnvalue))

(event Input|KeyboardEvents|DebugKey4
  (params (Key :type Key%20Structure :default "None") (ActionValue :type Input%20Action%20Value%20Structure))
  (:Pressed
    (CallFunction|SetNight)
    (Development|PrintString "Hello")))

(event Input|KeyboardEvents|DebugKey1
  (params (Key :type Key%20Structure :default "None") (ActionValue :type Input%20Action%20Value%20Structure))
  (:Pressed
    (CallFunction|SetMorning)
    (Development|PrintString "Hello")))

(event Input|KeyboardEvents|DebugKey2
  (params (Key :type Key%20Structure :default "None") (ActionValue :type Input%20Action%20Value%20Structure))
  (:Pressed
    (CallFunction|SetAfternoon)
    (Development|PrintString "Hello")))

(event Input|KeyboardEvents|DebugKey3
  (params (Key :type Key%20Structure :default "None") (ActionValue :type Input%20Action%20Value%20Structure))
  (:Pressed
    (CallFunction|SetEvening)
    (Development|PrintString "Hello")))

(fn ConstructionScript)

(fn SetMorning
  (bind _directionallight_ref (Variables|Default|GetDirectionalLight_Ref))
  (Transformation|SetActorRotation _directionallight_ref "0.000000,0.000000,30.000000")
  (Rendering|Components|Light|SetIntensity (Variables|/Script/Engine.Light|GetLightComponent _directionallight_ref) 3.5))

(fn SetAfternoon
  (bind _directionallight_ref (Variables|Default|GetDirectionalLight_Ref))
  (Transformation|SetActorRotation _directionallight_ref "0.000000,0.000000,90.000000")
  (Rendering|Components|Light|SetIntensity (Variables|/Script/Engine.Light|GetLightComponent _directionallight_ref) 5.0))

(fn SetEvening
  (bind _directionallight_ref (Variables|Default|GetDirectionalLight_Ref))
  (Transformation|SetActorRotation _directionallight_ref "0.000000,0.000000,160.000000")
  (Rendering|Components|Light|SetIntensity (Variables|/Script/Engine.Light|GetLightComponent _directionallight_ref) 2.5))

(fn SetNight
  (bind _directionallight_ref (Variables|Default|GetDirectionalLight_Ref))
  (Transformation|SetActorRotation _directionallight_ref "0.000000,0.000000,-90.000000")
  (Rendering|Components|Light|SetIntensity (Variables|/Script/Engine.Light|GetLightComponent _directionallight_ref) 0.0))