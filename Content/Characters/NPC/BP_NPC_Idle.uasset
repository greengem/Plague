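; BP_NPC_Idle is an interactable NPC that the player can talk to through a short hold-to-interact.
; Interact stores the instigator and opens a conversation on the DialogueJeff object, and ConversationClosed sends a closed message back to that instigator.
; SetOutlineState toggles the name text and the mesh's custom depth rendering together to highlight the character.
; The interact prompt still uses a placeholder character name.
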(event `/Game/Components/InteractionSystem/BPI_Interact.Interact`
  (params (Instigator :type "Actor Object Reference"))
  (set `self.InteractInstigator` Instigator)
  (`/Game/Components/DialogueSystem/Dialogue_Base.OpenConversation` (`self.Dialogue_Jeff`)))

(event `/Game/Components/DialogueSystem/BPI_Conversation.ConversationClosed`
  (message `/Game/Components/DialogueSystem/BPI_Conversation.ConversationClosed` (`self.InteractInstigator`)))

(event `/Game/Components/InteractionSystem/BPI_Interact.SetOutlineState`
  (params (`bShow?` :type Boolean))
  (bind _txt_charactername (`self.TXT_CharacterName`))
  (bind _mesh (`self.Mesh`))
  (if `bShow?`
    (`SceneComponent.SetVisibility` _txt_charactername true false)
    (`PrimitiveComponent.SetRenderCustomDepth` _mesh true)
    (else
      (`SceneComponent.SetVisibility` _txt_charactername false false)
      (`PrimitiveComponent.SetRenderCustomDepth` _mesh false))))

(fn `GetInteractHoldTime`
  (returns (HoldTime :type "Float (double-precision)"))
  (return 0.5))

(fn `GetInteractText`
  (returns (InteractText :type Text))
  (return "Talk to Character Name"))

(fn `UserConstructionScript`
  (`parent.UserConstructionScript`))