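; Melee enemy NPC Blueprint that handles sword attacks and drawing or sheathing a sword.
; Attack plays a slash montage and signals attack end on completion or interruption.
; Equip and Unequip play montages whose notifies spawn and attach the sword to a hand socket or destroy it, updating the wielding flag.
; Montage completion fires the equipped and unequipped callbacks.
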(event `/Game/Characters/NPC/AI/BPI_EnemyAI.Attack`
  ;[0 1 0.1301] NPC Attack Event
  (`|PlayMontage` (`self.Mesh`) "/Game/Characters/Animations/Mixamo/Melee/SwordSlash_Montage.SwordSlash_Montage"
    (:`OnCompleted`
      _)
    (:`OnInterrupted`
      _))
  (`self.OnAttackEnd`))

(event `/Game/Characters/NPC/AI/BPI_EnemyAI.EquipWeapon`
  ;[0 1 0.1301] NPC Equip Weapon
  (bind _notifyname (`|PlayMontage` (`self.Mesh`) "/Game/Characters/Animations/Mixamo/Melee/DrawSword_Montage.DrawSword_Montage")
    (:`OnCompleted`
      (`self.OnWeaponEquipped`))
    (:`OnNotifyBegin`
      (switch `name` _notifyname
        (:`DrawSword`
          (bind _returnvalue (`|SpawnActorFromClass` "/Game/Actors/BP_Weapon_Sword.BP_Weapon_Sword_C" (`self.GetTransform`) "Undefined" "MultiplyWithRoot" null null))
          (bind _output_get (set `self.WeaponActor` _returnvalue))
          (`self.K2_AttachToComponent` _output_get (`self.Mesh`) "hand_r_sword_socket" "SnapToTarget" "SnapToTarget" "SnapToTarget" true)
          (set `self.IsWieldingWeapon` true))))))

(event `/Game/Characters/NPC/AI/BPI_EnemyAI.UnequipWeapon`
  ;[0 1 0.1301] NPC Unequip Weapon
  (bind _notifyname (`|PlayMontage` (`self.Mesh`) "/Game/Characters/Animations/Mixamo/Melee/SheathSword_Montage.SheathSword_Montage")
    (:`OnCompleted`
      (`self.OnWeaponUnequipped`))
    (:`OnNotifyBegin`
      (switch `name` _notifyname
        (:`DropSword`
          (`self.K2_DestroyActor` (`self.WeaponActor`))
          (set `self.IsWieldingWeapon` false))))))

(fn `UserConstructionScript`
  (`parent.UserConstructionScript`))