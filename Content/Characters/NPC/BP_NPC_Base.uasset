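; Base NPC character Blueprint that supplies health, patrol route, combat ranges and movement speed to its AI, and supports dialogue interaction.
; BeginPlay caches the AIC_Enemy_Base controller and creates an overhead health bar widget bound to itself.
; On death it stops the AI brain, flags the controller dead, hides the bar and ragdolls the mesh.
; Dialogue events toggle the name text and notify the interacting instigator when conversation closes.
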(event `self.ReceiveBeginPlay`
  ;[1 0.2961 0.1274] Get Reference to AI Controller Class
  (bind _asaic_enemy_base (cast `/Game/Characters/NPC/AI/AIC_Enemy_Base` (`AIBlueprintHelperLibrary.GetAIController` self)))
  (set `self.AIC Enemy Base` _asaic_enemy_base)
  ;[1 0.2961 0.1274] Show Health Bar Above NPC
  (bind _returnvalue (`|CreateWidget` "/Game/UI/Game/WB_NPC_HealthBar.WB_NPC_HealthBar_C" null self))
  (`WidgetComponent.SetWidget` (`self.HealthBar`) _returnvalue))

(event `/Game/Components/HealthSystem/BPI_Health.OnKilled`
  (params (DamageInstigator :type "Controller Object Reference") (DamageCauser :type "Actor Object Reference"))
  (bind _mesh (`self.Mesh`))
  ;[1 0.2961 0.1274] NPC Death Event
  (`self.StopAnimMontage` null)
  (`BrainComponent.StopLogic` (`AIController.BrainComponent` (`self.AIC Enemy Base`)) "") ; Turn the Brain off!
  (`/Game/Characters/NPC/AI/AIC_Enemy_Base.SetStateAsDead` (`self.AIC Enemy Base`))
  (`SceneComponent.SetVisibility` (`self.HealthBar`) false true)
  (`PrimitiveComponent.SetSimulatePhysics` _mesh true)
  (`PrimitiveComponent.SetCollisionEnabled` _mesh "QueryAndPhysics"))

(event `/Game/Interactable/BPI_Interact.Dialogue_SetInteractableState`
  (params (`bCanShowInteract?` :type Boolean))
  (if `bCanShowInteract?`
    (`SceneComponent.SetVisibility` (`self.TXT_CharacterName`) true false)
    (else
      (`SceneComponent.SetVisibility` (`self.TXT_CharacterName`) false false))))

(event `/Game/Interactable/BPI_Interact.Dialogue_ConversationClosed`
  (message `/Game/Interactable/BPI_Interact.Dialogue_ConversationClosed` (`self.InteractInstigator`)))

(fn `Container_LookAt`
  (returns (Message :type Text))
  (return ""))

(fn `GetCurrentHealth`
  (returns (Health :type "Float (double-precision)"))
  (return (`/Game/Components/HealthSystem/HealthSystem.Health_Current` (`self.HealthSystem`))))

(fn `GetIdealRange`
  (returns (AttackRadius :type "Float (double-precision)") (DefendRadius :type "Float (double-precision)"))
  (return 150.0 350.0))

(fn `GetMaxHealth`
  (returns (MaxHealth :type "Float (double-precision)"))
  (return (`/Game/Components/HealthSystem/HealthSystem.Health_Max` (`self.HealthSystem`))))

(fn `GetPatrolRoute`
  (returns (NewParam :type "/Game/Characters/NPC/AI/BP_PatrolRoute_Parent Object Reference"))
  (return (`self.PatrolRoute`)))

(fn `Heal`
  (params (Amount :type "Float (double-precision)"))
  (returns (NewHealth :type "Float (double-precision)"))
  (return 0.0))

(fn `SetMovementSpeed`
  (params (Speed :type "/Game/Characters/NPC/AI/Enums/E_MovementSpeed Enum" :default "NewEnumerator0"))
  (returns (SpeedValue :type "Float (double-precision)"))
  (bind _output_get (set `CharacterMovementComponent.MaxWalkSpeed` (select `/Game/Characters/NPC/AI/Enums/E_MovementSpeed` Speed :`NewEnumerator1` 150.0 :`NewEnumerator2` 300.0 :`NewEnumerator3` 400.0 :!type "Float (single-precision)") (`self.CharacterMovement`)))
  (return _output_get))

(fn `UserConstructionScript`
  (`TextRenderComponent.K2_SetText` (`self.TXT_CharacterName`) (`self.CharacterName`)))