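; Player controller for gameplay that mounts the HUD on BeginPlay and hides the cursor with game-only input.
; The pause action creates the pause menu with UI-only input and a visible cursor, or removes an existing one, restores game input and forces garbage collection.
; The inventory action uses a FlipFlop to alternately show and remove the inventory menu through the HUD widget.
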(event `self.ReceiveBeginPlay`
  ;[0.956 0.4233 1] Mount in Game HUD and create Reference
  (bind _returnvalue (`|CreateWidget` "/Game/UI/Game/WB_HUD.WB_HUD_C" self))
  (bind _output_get (set `self.WB_HUD` _returnvalue))
  (`UserWidget.AddToViewport` _output_get 0)
  ;[0.956 0.4233 1] Hide Mouse and set input to Game Only
  (`WidgetBlueprintLibrary.SetInputMode_GameOnly` self)
  (set `self.bShowMouseCursor` false))

(event `EnhancedInput|/Game/Input/Actions/IA_Pause`
  (params (ActionValue :type Boolean) (ElapsedSeconds :type "Float (double-precision)") (TriggeredSeconds :type "Float (double-precision)") (InputAction :type "InputAction Object Reference" :default "/Game/Input/Actions/IA_Pause.IA_Pause"))
  (bind _returnvalue (`GameplayStatics.GetPlayerController` 0))
  ;[0.956 0.4233 1] Pause Menu Toggling
  (:`Started`
    (`self.WB_PauseMenu`
      (:`then`
        (bind _foundwidgets (`WidgetBlueprintLibrary.GetAllWidgetsOfClass` "/Game/UI/Pause/WB_PauseMenu.WB_PauseMenu_C"))
        (`Widget.RemoveFromParent` (`|GetArrayItem` _foundwidgets))
        (`WidgetBlueprintLibrary.SetInputMode_GameOnly` _returnvalue)
        (set `PlayerController.bShowMouseCursor` false _returnvalue)
        (set `self.WB_PauseMenu` null)
        (`KismetSystemLibrary.CollectGarbage`))
      (:`else`
        (bind _returnvalue_2 (`|CreateWidget` "/Game/UI/Pause/WB_PauseMenu.WB_PauseMenu_C" _returnvalue))
        (bind _output_get (set `self.WB_PauseMenu` _returnvalue_2))
        (`UserWidget.AddToViewport` _output_get 0)
        (`WidgetBlueprintLibrary.SetInputMode_UIOnlyEx` _returnvalue _output_get)
        (set `PlayerController.bShowMouseCursor` true _returnvalue)))))

(event `EnhancedInput|/Game/Input/Actions/IA_Inventory`
  (params (ActionValue :type Boolean) (ElapsedSeconds :type "Float (double-precision)") (TriggeredSeconds :type "Float (double-precision)") (InputAction :type "InputAction Object Reference" :default "/Game/Input/Actions/IA_Inventory.IA_Inventory"))
  (bind _wb_hud (`self.WB_HUD`))
  ;[0.956 0.4233 1] Inventory Menu Toggling
  (:`Started`
    (`/Engine/EditorBlueprintResources/StandardMacros.FlipFlop`
      (:`A`
        (`/Game/UI/Game/WB_HUD.DisplayInventoryMenu` _wb_hud))
      (:`B`
        (`/Game/UI/Game/WB_HUD.RemoveInventoryMenu` _wb_hud)))))

(fn `UserConstructionScript`)